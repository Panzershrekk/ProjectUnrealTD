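; BP_GameManager handles mouse-driven tower buying and placement, showing the cursor at game start.
; A tower-selection delegate bound on BeginPlay spawns or despawns a ghost tower depending on whether placement is active.
; Tick moves the ghost to the Visibility trace hit under the cursor.
; During placement, left click buys and spawns the selected tower at the ghost's location, and right click cancels the selection.
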(event `self.ReceiveBeginPlay`
  (`|ExecutionSequence`
    (:`then_1`
      (set `self.bShowMouseCursor` true))
    (:`then_2`
      (add `self.OnSelectTowerToBuy` (delegate `OnSelectTowerToBuy_Événement`)))))

(event `OnSelectTowerToBuy_Événement`
  (if (`self.IsTowerBeingPlaced`)
    (`self.SpawnGhostTower`)
    (else
      (`self.DespawnGhostTower`))))

(event `self.ReceiveTick`
  (params (DeltaSeconds :type "Float (single-precision)"))
  (`/Engine/EditorBlueprintResources/StandardMacros.IsValid` (`self.GhostTower`)
    (:`Is Valid`
      (`self.K2_SetActorLocation` (`self.GhostTower`) (`.Location` (`GameplayStatics.BreakHitResult` (`self.GetHitResultUnderCursorByChannel` "TraceTypeQuery1"))) false false))))

(event `Key|LeftMouseButton`
  (params (Key :type "Key Structure"))
  (:`Pressed`
    (if (`self.IsTowerBeingPlaced`)
      (`self.BuyAndSpawnSelectedTower` (`self.K2_GetActorLocation` (`self.GhostTower`))))))

(event `Key|RightMouseButton`
  (params (Key :type "Key Structure"))
  (:`Pressed`
    (if (`self.IsTowerBeingPlaced`)
      (`self.CancelBuyableTowerSelection`))))

(fn `UserConstructionScript`)